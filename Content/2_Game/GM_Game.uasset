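; Game mode for a team-based game that spawns players by team, tracks team scores and handles victory.
; Controllers are queued at login, then after a short delay spawned and possessed at team locations using the game instance's Composition, matched by controller ID.
; Default pawn spawning is overridden empty.
; AddScore broadcasts score changes and, once a team reaches the threshold, shows the victory widget and disables all players' input.
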(event `self.K2_PostLogin`
  (params (NewPlayer :type "PlayerController Object Reference"))
  (`KismetArrayLibrary.Array_Add` (`self.Queue`) NewPlayer))

(event `self.ReceiveBeginPlay`
  (`|ExecutionSequence`
    (:`then_0`
      (bind _returnvalue (`|CreateWidget` "/Game/2_Game/HUD/WBP_game.WBP_game_C" (`GameplayStatics.GetPlayerController` 0)))
      (bind _output_get (set `self.WBP_Game` _returnvalue))
      (`UserWidget.AddToViewport` _output_get 0))
    (:`then_1`
      (bind _asgi_game (cast `/Game/0_Generic/GI_Game` (`GameplayStatics.GetGameInstance`)))
      (set `self.GI` _asgi_game))
    (:`then_2`
      (`KismetSystemLibrary.Delay` 2.0)
      (for _array_element (`self.Queue`)
        (`self.SpawnPlayer` _array_element)))))

(fn `AddScore`
  (params (Team :type "/Game/0_Generic/ENUM_Teams Enum" :default "NewEnumerator0") (ScoreToAdd :type Integer))
  (bind _scorring (`self.Scorring`))
  (`BlueprintMapLibrary.Map_Add` _scorring Team (+ (`BlueprintMapLibrary.Map_Find` (`self.Scorring`) Team) ScoreToAdd))
  (`self.ED_OnChangeScrorring` _scorring)
  (if (>= (`BlueprintMapLibrary.Map_Find` (`self.Scorring`) Team) 1)
    (`|ExecutionSequence`
      (:`then_0`
        (bind _returnvalue (`|CreateWidget` "/Game/2_Game/HUD/WBP_VIctory.WBP_VIctory_C" (`GameplayStatics.GetPlayerController` 0) Team))
        (`UserWidget.AddToViewport` _returnvalue 1))
      (:`then_1`
        (bind _outactors (`GameplayStatics.GetAllActorsOfClass` "/Script/Engine.PlayerController"))
        (for _array_element _outactors
          (`self.DisableInput` _array_element _array_element))))))

(fn `SpawnDefaultPawnAtTransform`
  (params (NewPlayer :type "Controller Object Reference") (SpawnTransform :type "Transform Structure (by ref)"))
  (returns (ReturnValue :type "Pawn Object Reference")))

(fn `SpawnPlayer`
  (params (PC :type "PlayerController Object Reference"))
  (for _array_element (`/Game/0_Generic/GI_Game.Composition` (`self.GI`))
    (bind (_playerindex _team) (break `/Game/0_Generic/Composition` _array_element))
    (if (== _playerindex (`GameplayStatics.GetPlayerControllerID` PC))
      (bind (_value _returnvalue) (`BlueprintMapLibrary.Map_Find` (`self.SpawnLocation`) _team))
      (`KismetSystemLibrary.PrintString` (`KismetStringLibrary.Conv_BoolToString` _returnvalue))
      (bind _returnvalue_2 (`|SpawnActorFromClass` "/Game/2_Game/Pawn/Player/CHAR_Player.CHAR_Player_C" (`KismetMathLibrary.MakeTransform` _value) "Undefined" "MultiplyWithRoot" PC null))
      (`Controller.Possess` PC _returnvalue_2)
      (`KismetSystemLibrary.PrintString` (`KismetStringLibrary.Concat_StrStr` "Spawn Player index : " (`KismetStringLibrary.Conv_IntToString` _playerindex) "At location  :" (`KismetStringLibrary.Conv_VectorToString` _value))))))

(fn `UserConstructionScript`)
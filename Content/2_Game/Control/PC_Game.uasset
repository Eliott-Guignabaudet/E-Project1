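; PC_Game is a player controller that shows the game through a level camera and drives the controlled pawn.
; On BeginPlay and again on possession, it sets the view target to the first CameraActor found in the level.
; MoveX and MoveY axes pass a deadzone check, then move the pawn along fixed world axes, Y and X respectively.
; The Dash action calls Dash on the pawn when it is a CHAR_Player.
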(event `self.ReceiveBeginPlay`
  (bind _outactors (`GameplayStatics.GetAllActorsOfClass` "/Script/Engine.CameraActor" :!label _label))
  (`self.SetViewTargetWithBlend` self (`|GetArrayItem` _outactors) 0.0 "VTBlend_Linear" 0.0 false))

(event `self.ReceivePossess`
  (params (PossessedPawn :type "Pawn Object Reference"))
  (goto _label))

(event `Key|Pause`
  (params (Key :type "Key Structure")))

(event `InputAxis|MoveX`
  (params (AxisValue :type "Float (single-precision)"))
  (if (> (`KismetMathLibrary.Abs` AxisValue) 0.25)
    (`/Engine/EditorBlueprintResources/StandardMacros.IsValid` (`self.K2_GetPawn` self)
      (:`Is Valid`
        (`Pawn.AddMovementInput` (`self.K2_GetPawn` self) (`KismetMathLibrary.MakeVector` 0.0 AxisValue) 1.0 false)))))

(event `InputAxis|MoveY`
  (params (AxisValue :type "Float (single-precision)"))
  (if (> (`KismetMathLibrary.Abs` AxisValue) 0.25)
    (`/Engine/EditorBlueprintResources/StandardMacros.IsValid` (`self.K2_GetPawn` self)
      (:`Is Valid`
        (`Pawn.AddMovementInput` (`self.K2_GetPawn` self) (`KismetMathLibrary.MakeVector` AxisValue) 1.0 false)))))

(event `InputAction|Dash`
  (params (Key :type "Key Structure"))
  (:`Pressed`
    (bind _aschar_player (cast `/Game/2_Game/Pawn/Player/CHAR_Player` (`self.K2_GetPawn` self)))
    (`/Game/2_Game/Pawn/Player/CHAR_Player.Dash` _aschar_player)))

(fn `UserConstructionScript`)
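; PC_Menu is the menu player controller, turning input actions into avatar and team changes.
; On begin play it sets Game and UI input mode and caches the GI_Game game instance.
; Input actions call that instance to cycle the avatar or switch this controller to one of four coloured teams.
; Only the yellow team action checks that the pressed key is a gamepad key.
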(event `self.ReceiveBeginPlay`
  ;[0.2263 1 0] CONTRUCT
  (`|ExecutionSequence`
    (:`then_0`
      (`WidgetBlueprintLibrary.SetInputMode_GameAndUIEx` self null "DoNotLock" false))
    (:`then_1`
      (bind _asgi_game (cast `/Game/0_Generic/GI_Game` (`GameplayStatics.GetGameInstance`)))
      (set `self.GI` _asgi_game))))

(event `InputAction|NavigateYellowTeam`
  (params (Key :type "Key Structure"))
  ;[1 1 1] Switch Team
  (:`Pressed`
    (if (`KismetInputLibrary.Key_IsGamepadKey` Key)
      (`/Game/0_Generic/GI_Game.SwitchTeam` (`self.GI`) self "NewEnumerator0"))))

(event `InputAction|NextAvatar`
  (params (Key :type "Key Structure"))
  ;[1 1 1] Next Avatar
  (:`Pressed`
    (`/Game/0_Generic/GI_Game.ChangeAvatar` (`self.GI`) self)))

(event `InputAction|NavigateRedTeam`
  (params (Key :type "Key Structure"))
  ;[1 1 1] Switch Team
  (:`Pressed`
    (`/Game/0_Generic/GI_Game.SwitchTeam` (`self.GI`) self "NewEnumerator1")))

(event `InputAction|NavigateGreenTeam`
  (params (Key :type "Key Structure"))
  ;[1 1 1] Switch Team
  (:`Pressed`
    (`/Game/0_Generic/GI_Game.SwitchTeam` (`self.GI`) self "NewEnumerator2")))

(event `InputAction|NavigateBlueTeam`
  (params (Key :type "Key Structure"))
  ;[1 1 1] Switch Team
  (:`Pressed`
    (`/Game/0_Generic/GI_Game.SwitchTeam` (`self.GI`) self "NewEnumerator3")))

(fn `UserConstructionScript`)